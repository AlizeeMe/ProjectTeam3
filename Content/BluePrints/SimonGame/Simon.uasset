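; Simon memory mini-game actor with four clickable colored spheres, lights and sounds.
; A random sequence is generated at start, and GamePhase replays the growing Progress array through a delayed-loop macro while input is locked.
; Sphere clicks are checked step by step; success extends the sequence, while a mistake restarts with a new one.
; Completing the full sequence plays a final animation and flags completion on Mouse_GameMode and StoreDatas.
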(event `self.ShereBlue.OnClicked`
  (params (TouchedComponent :type "PrimitiveComponent Object Reference") (ButtonPressed :type "Key Structure"))
  (bind _witchstage (`self.WitchStage`))
  ;[0.9202 1 0.9012] Dectection click on shere
  (if (not (`self.NoInterractWithSystem`))
    ;[1 0.2317 0.8643] Test the validity of the color selected
    (if (== (`|GetArrayItem` (`self.Progress`) (`self.PlayerStage`)) (`self.Blue`))
      (set `self.NoInterractWithSystem` true)
      ;[1 0.9607 0.3615] Trun on the light selected for a short periode
      (`GameplayStatics.PlaySoundAtLocation` "/Game/BluePrints/SimonGame/Music/Blue.Blue" (0.0 0.0 0.0) (struct) 1.0 1.0 0.0 null null null)
      (`SceneComponent.SetVisibility` (`self.BlueLight`) true false)
      (`KismetSystemLibrary.Delay` 0.5)
      (`self.TurnOffLight` :!label _label)
      ;[0.1963 0.4324 1] Test if more stage as to be add or not and continue
      (if (== (`self.PlayerStage`) (`self.WitchStage`))
        (set `self.PlayerStage` 0)
        ;[0.00063 0 1] End of Simon Game + Final animation
        (if (== (+ _witchstage 1) (`self.MaxRangeSimon`))
          (`self.FinalAnimation`
            (:`Exec`
              (`self.EndGame`)))
          (else
            (bind _result (`/Engine/EditorBlueprintResources/StandardMacros.IncrementInt` _witchstage)
              (:`  `
                (bind _output_get (set `self.WitchStage` _result))
                (`self.AddValueToProgress` _output_get)
                (`KismetSystemLibrary.Delay` 1.3)
                (`self.GamePhase` (`self.Progress`))))))
        (else
          (bind _result_2 (`/Engine/EditorBlueprintResources/StandardMacros.IncrementInt` (`self.PlayerStage`))
            (:`  `
              (set `self.PlayerStage` _result_2)
              (set `self.NoInterractWithSystem` false)))))
      (else
        (`self.TurnOffLight`)
        ;[1 0.03125 0.03125] Fail color, special annimation and reloaed
        (`GameplayStatics.PlaySoundAtLocation` "/Game/BluePrints/SimonGame/Music/Fail.Fail" (0.0 0.0 0.0) (struct) 1.0 1.0 0.0 null null null :!label _label_2)
        (`self.CustomLoopwithDelay` (`self.SimonRandomArray`)
          (:`LoopBody`
            (`self.TurnOnLight`))
          (:`Complet`
            (`self.TurnOffLight`)
            (`KismetArrayLibrary.Array_Clear` (`self.SimonRandomArray`))
            (`KismetArrayLibrary.Array_Clear` (`self.Progress`))
            (set `self.WitchStage` 0)
            (set `self.PlayerStage` 0)
            (`self.GenerateSimon`)
            (`self.AddValueToProgress` 0)
            (`self.GamePhase` (`self.Progress`))))))))

(event `self.ShereGreen.OnClicked`
  (params (TouchedComponent :type "PrimitiveComponent Object Reference") (ButtonPressed :type "Key Structure"))
  ;[0.9202 1 0.9012] Dectection click on shere
  (if (not (`self.NoInterractWithSystem`))
    ;[1 0.2317 0.8643] Test the validity of the color selected
    (if (== (`|GetArrayItem` (`self.Progress`) (`self.PlayerStage`)) (`self.Green`))
      (set `self.NoInterractWithSystem` true)
      ;[1 0.9607 0.3615] Trun on the light selected for a short periode
      (`GameplayStatics.PlaySoundAtLocation` "/Game/BluePrints/SimonGame/Music/Green.Green" (0.0 0.0 0.0) (struct) 1.0 1.0 0.0 null null null)
      (`SceneComponent.SetVisibility` (`self.GreenLight`) true false)
      (`KismetSystemLibrary.Delay` 0.5)
      (goto _label)
      (else
        (`self.TurnOffLight`)
        (goto _label_2)))))

(event `self.ShereRed.OnClicked`
  (params (TouchedComponent :type "PrimitiveComponent Object Reference") (ButtonPressed :type "Key Structure"))
  ;[0.9202 1 0.9012] Dectection click on shere
  (if (not (`self.NoInterractWithSystem`))
    ;[1 0.2317 0.8643] Test the validity of the color selected
    (if (== (`|GetArrayItem` (`self.Progress`) (`self.PlayerStage`)) (`self.Red`))
      (set `self.NoInterractWithSystem` true)
      ;[1 0.9607 0.3615] Trun on the light selected for a short periode
      (`GameplayStatics.PlaySoundAtLocation` "/Game/BluePrints/SimonGame/Music/Red.Red" (0.0 0.0 0.0) (struct) 1.0 1.0 0.0 null null null)
      (`SceneComponent.SetVisibility` (`self.RedLight`) true false)
      (`KismetSystemLibrary.Delay` 0.5)
      (goto _label)
      (else
        (`self.TurnOffLight`)
        (goto _label_2)))))

(event `self.ShereYellow.OnClicked`
  (params (TouchedComponent :type "PrimitiveComponent Object Reference") (ButtonPressed :type "Key Structure"))
  ;[0.9202 1 0.9012] Dectection click on shere
  (if (not (`self.NoInterractWithSystem`))
    ;[1 0.2317 0.8643] Test the validity of the color selected
    (if (== (`|GetArrayItem` (`self.Progress`) (`self.PlayerStage`)) (`self.Yellow`))
      (set `self.NoInterractWithSystem` true)
      ;[1 0.9607 0.3615] Trun on the light selected for a short periode
      (`GameplayStatics.PlaySoundAtLocation` "/Game/BluePrints/SimonGame/Music/Yellow.Yellow" (0.0 0.0 0.0) (struct) 1.0 1.0 0.0 null null null)
      (`SceneComponent.SetVisibility` (`self.YellowLight`) true false)
      (`KismetSystemLibrary.Delay` 0.5)
      (goto _label)
      (else
        (`self.TurnOffLight`)
        (goto _label_2)))))

(event `self.ReceiveBeginPlay`
  ;[0.2188 1 1] Start game, and initialyse ramdom for simon
  (set `self.NoInterractWithSystem` true)
  (`self.GenerateSimon`)
  (set `self.ClickBlue` false)
  (set `self.ClickYellow` false)
  (set `self.ClickGreen` false)
  (set `self.ClickRed` false)
  (set `self.Blue` 1)
  (set `self.Yellow` 2)
  (set `self.Green` 4)
  (set `self.Red` 3)
  (`self.AddValueToProgress` 0)
  (`self.GamePhase` (`self.Progress`)))

(fn `AddValueToProgress`
  (params (Index :type Integer))
  (`KismetArrayLibrary.Array_Add` (`self.Progress`) (`|GetArrayItem` (`self.SimonRandomArray`) Index)))

(fn `BrowseSimon`
  (set `self.Blue` 1)
  (set `self.Yellow` 2)
  (set `self.Green` 3)
  (set `self.Red` 4)
  (for _array_element (`self.SimonRandomArray`)
    (if (== _array_element (`self.Blue`))
      (`SceneComponent.SetVisibility` (`self.BlueLight`) true false)
      (elif (== _array_element (`self.Yellow`))
        (`SceneComponent.SetVisibility` (`self.YellowLight`) true false)
        (elif (== _array_element (`self.Red`))
          (`SceneComponent.SetVisibility` (`self.RedLight`) true false)
          (elif (== _array_element (`self.Green`))
            (`SceneComponent.SetVisibility` (`self.GreenLight`) true false)))))))

(fn `EndGame`
  ;[1 1 1] Update the booleen is finish of the game
  (bind _asmouse_game_mode (cast `/Game/BluePrints/SimonGame/Mouse_GameMode` (`GameplayStatics.GetGameMode`)))
  (set `/Game/BluePrints/SimonGame/Mouse_GameMode.IsFinish` true _asmouse_game_mode)
  ;[0.08507 0.5104 0.2683] Update game instance
  (bind _asstore_datas (cast `/Game/Assets/Room/StoreDatas` (`GameplayStatics.GetGameInstance`)))
  (set `/Game/Assets/Room/StoreDatas.IsSimonFinished` true _asstore_datas))

(fn `GenerateSimon`
  ;[0.9151 0.2163 1] Set max range
  (bind _output_get (set `self.MaxRangeSimon` 7))
  ;[0.3279 0.2965 1] While MaxRange not equal to the size of our random array we add new random number to SimonRandomArray
  (while (!= (`self.Iter`) _output_get)
    (bind _result (`/Engine/EditorBlueprintResources/StandardMacros.IncrementInt` (`self.Iter`))
      (:`  `
        (set `self.Iter` _result)
        (bind _output_get_2 (set `self.RandomTest` (`KismetMathLibrary.RandomIntegerInRange` 1 4)))
        (`KismetArrayLibrary.Array_Add` (`self.SimonRandomArray`) _output_get_2)
        (for _ (`self.SimonRandomArray`)
          _))))
  (set `self.Iter` 0))

(fn `TurnOffLight`
  ;[0.162 1 0.2301] Turn off all the light
  (`SceneComponent.SetVisibility` (`self.BlueLight`) false false)
  (`SceneComponent.SetVisibility` (`self.YellowLight`) false false)
  (`SceneComponent.SetVisibility` (`self.RedLight`) false false)
  (`SceneComponent.SetVisibility` (`self.GreenLight`) false false))

(fn `TurnOnLight`
  ;[1 0.1409 0.08121] Turn on all the light
  (`SceneComponent.SetVisibility` (`self.BlueLight`) true false)
  (`SceneComponent.SetVisibility` (`self.YellowLight`) true false)
  (`SceneComponent.SetVisibility` (`self.RedLight`) true false)
  (`SceneComponent.SetVisibility` (`self.GreenLight`) true false))

(fn `UserConstructionScript`)