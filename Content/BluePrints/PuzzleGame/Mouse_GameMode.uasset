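; Game mode for a mouse puzzle game that keeps an elapsed play timer and shows the end screen when the game finishes.
; Tick runs through a one-second Delay, so each pass increments seconds and rolls them over into minutes while IsFinish is false.
; Once IsFinish is set, it creates the EndWidget for player 0 and adds it to the viewport, guarded by a flag so it appears only once.
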(event `self.ReceiveBeginPlay`)

(event `self.ReceiveTick`
  (params (DeltaSeconds :type "Float (single-precision)"))
  (`KismetSystemLibrary.Delay` 1.0)
  ;[1 1 1] If the game is not finish inc timer
  (if (`self.isFinish`)
    ;[1 1 1] Display results only 1 time
    (if (not (`self.isResultsDisplayed`))
      (set `self.isResultsDisplayed` true)
      (bind _returnvalue (`|CreateWidget` "/Game/BluePrints/PuzzleGame/EndWidget.EndWidget_C" (`GameplayStatics.GetPlayerController` 0)))
      (`UserWidget.AddToViewport` _returnvalue 0))
    (else
      ;[1 1 1] This function is called each sec so increment sec each times
      (`/Engine/EditorBlueprintResources/StandardMacros.IncrementInt` (`self.TimeSec`)
        (:`  `
          ;[1 1 1] If sec > 59 it's a new min so inc min and reset sec
          (if (> (`self.TimeSec`) 59)
            (set `self.TimeSec` 0)
            (`/Engine/EditorBlueprintResources/StandardMacros.IncrementInt` (`self.TimeMin`))))))))

(fn `UserConstructionScript`)