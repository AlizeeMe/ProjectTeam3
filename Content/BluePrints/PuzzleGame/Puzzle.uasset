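; Sliding 15-puzzle actor: clicking a tile next to the free slot swaps it into that slot.
; The construction script records solved positions, then lays pieces out in a hand-picked solvable shuffle.
; Clicks check 4x4 grid adjacency from array indices, then swap both world locations and array entries.
; Tick compares the current array to the solved order and sets IsFinish on Mouse_GameMode when they match.
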(event `self.ReceiveBeginPlay`
  ;[1 1 1] Display the mouse in the game
  (set `PlayerController.bShowMouseCursor` true (`GameplayStatics.GetPlayerController` 0)))

(event `self.ReceiveTick`
  (params (DeltaSeconds :type "Float (single-precision)"))
  ;[1 1 1] Each frame check if game is finish
  (`self.IsFinish`))

(event `self.1.OnClicked`
  (params (TouchedComponent :type "PrimitiveComponent Object Reference") (ButtonPressed :type "Key Structure"))
  ;[1 1 1] Swap piece with free place when click on it
  (set `self.PieceToSwap` TouchedComponent)
  (`self.SwapFreeAndPiece`))

(event `self.2.OnClicked`
  (params (TouchedComponent :type "PrimitiveComponent Object Reference") (ButtonPressed :type "Key Structure"))
  ;[1 1 1] Swap piece with free place when click on it
  (set `self.PieceToSwap` TouchedComponent)
  (`self.SwapFreeAndPiece`))

(event `self.3.OnClicked`
  (params (TouchedComponent :type "PrimitiveComponent Object Reference") (ButtonPressed :type "Key Structure"))
  ;[1 1 1] Swap piece with free place when click on it
  (set `self.PieceToSwap` TouchedComponent)
  (`self.SwapFreeAndPiece`))

(event `self.4.OnClicked`
  (params (TouchedComponent :type "PrimitiveComponent Object Reference") (ButtonPressed :type "Key Structure"))
  ;[1 1 1] Swap piece with free place when click on it
  (set `self.PieceToSwap` TouchedComponent)
  (`self.SwapFreeAndPiece`))

(event `self.5.OnClicked`
  (params (TouchedComponent :type "PrimitiveComponent Object Reference") (ButtonPressed :type "Key Structure"))
  ;[1 1 1] Swap piece with free place when click on it
  (set `self.PieceToSwap` TouchedComponent)
  (`self.SwapFreeAndPiece`))

(event `self.6.OnClicked`
  (params (TouchedComponent :type "PrimitiveComponent Object Reference") (ButtonPressed :type "Key Structure"))
  ;[1 1 1] Swap piece with free place when click on it
  (set `self.PieceToSwap` TouchedComponent)
  (`self.SwapFreeAndPiece`))

(event `self.7.OnClicked`
  (params (TouchedComponent :type "PrimitiveComponent Object Reference") (ButtonPressed :type "Key Structure"))
  ;[1 1 1] Swap piece with free place when click on it
  (set `self.PieceToSwap` TouchedComponent)
  (`self.SwapFreeAndPiece`))

(event `self.8.OnClicked`
  (params (TouchedComponent :type "PrimitiveComponent Object Reference") (ButtonPressed :type "Key Structure"))
  ;[1 1 1] Swap piece with free place when click on it
  (set `self.PieceToSwap` TouchedComponent)
  (`self.SwapFreeAndPiece`))

(event `self.9.OnClicked`
  (params (TouchedComponent :type "PrimitiveComponent Object Reference") (ButtonPressed :type "Key Structure"))
  ;[1 1 1] Swap piece with free place when click on it
  (set `self.PieceToSwap` TouchedComponent)
  (`self.SwapFreeAndPiece`))

(event `self.10.OnClicked`
  (params (TouchedComponent :type "PrimitiveComponent Object Reference") (ButtonPressed :type "Key Structure"))
  ;[1 1 1] Swap piece with free place when click on it
  (set `self.PieceToSwap` TouchedComponent)
  (`self.SwapFreeAndPiece`))

(event `self.11.OnClicked`
  (params (TouchedComponent :type "PrimitiveComponent Object Reference") (ButtonPressed :type "Key Structure"))
  ;[1 1 1] Swap piece with free place when click on it
  (set `self.PieceToSwap` TouchedComponent)
  (`self.SwapFreeAndPiece`))

(event `self.12.OnClicked`
  (params (TouchedComponent :type "PrimitiveComponent Object Reference") (ButtonPressed :type "Key Structure"))
  ;[1 1 1] Swap piece with free place when click on it
  (set `self.PieceToSwap` TouchedComponent)
  (`self.SwapFreeAndPiece`))

(event `self.13.OnClicked`
  (params (TouchedComponent :type "PrimitiveComponent Object Reference") (ButtonPressed :type "Key Structure"))
  ;[1 1 1] Swap piece with free place when click on it
  (set `self.PieceToSwap` TouchedComponent)
  (`self.SwapFreeAndPiece`))

(event `self.14.OnClicked`
  (params (TouchedComponent :type "PrimitiveComponent Object Reference") (ButtonPressed :type "Key Structure"))
  ;[1 1 1] Swap piece with free place when click on it
  (set `self.PieceToSwap` TouchedComponent)
  (`self.SwapFreeAndPiece`))

(event `self.15.OnClicked`
  (params (TouchedComponent :type "PrimitiveComponent Object Reference") (ButtonPressed :type "Key Structure"))
  ;[1 1 1] Swap piece with free place when click on it
  (set `self.PieceToSwap` TouchedComponent)
  (`self.SwapFreeAndPiece`))

(fn `IsFinish`
  ;[1 1 1] Check if the actual position of pieces are the good ones
  (if (`KismetArrayLibrary.Array_Identical` (`self.ArrayPiecesOrdered`) (`self.ArrayPieces`))
    ;[1 1 1] Update the booleen is finish of the game
    (bind _asmouse_game_mode (cast `/Game/BluePrints/PuzzleGame/Mouse_GameMode` (`GameplayStatics.GetGameMode`)))
    (set `/Game/BluePrints/PuzzleGame/Mouse_GameMode.isFinish` true _asmouse_game_mode)))

(fn `IsNeighbour`
  (bind _returnvalue (`KismetArrayLibrary.Array_Find` (`self.ArrayPieces`) (`self.FREE`)))
  ;[1 1 1] Get coordinates of the piece to swap
  (bind _asstatic_mesh_component (cast `StaticMeshComponent` (`self.PieceToSwap`)))
  (bind _returnvalue_2 (`KismetArrayLibrary.Array_Find` (`self.ArrayPieces`) _asstatic_mesh_component))
  (set `self.TempX` (mod _returnvalue_2 4))
  (set `self.TempY` (/ _returnvalue_2 4))
  ;[1 1 1] Get Coordinates of the free place
  (set `self.TempFreeX` (mod _returnvalue 4))
  (set `self.TempFreeY` (/ _returnvalue 4))
  ;[1 1 1] Compute difference on X
  (set `self.DiffX` (`KismetMathLibrary.Abs_Int` (- (`self.TempX`) (`self.TempFreeX`))))
  ;[1 1 1] Compute Y diff
  (set `self.DiffY` (`KismetMathLibrary.Abs_Int` (- (`self.TempY`) (`self.TempFreeY`))))
  ;[1 1 1] If diff X = 1, Diff Y have to be 0. Else if diff X = 0  Diff Y have to be 1
  (if (>= (`self.DiffX`) 1)
    (if (== (`self.DiffX`) 1)
      (if (== (`self.DiffY`) 0)
        (set `self.b_isNeighboor` true)
        (else
          (set `self.b_isNeighboor` false)))
      (else
        (set `self.b_isNeighboor` false)))
    (elif (>= (`self.DiffY`) 1)
      (if (== (`self.DiffY`) 1)
        (set `self.b_isNeighboor` true)
        (else
          (set `self.b_isNeighboor` false)))
      (else
        (set `self.b_isNeighboor` false)))))

(fn `SwapFreeAndPiece`
  (bind _piecetoswap (`self.PieceToSwap`))
  (`self.IsNeighbour`)
  (if (`self.b_isNeighboor`)
    ;[1 1 1] Set Temp var to be able to swap the 2 pieces
    (set `self.LocationFreePlace` (`SceneComponent.K2_GetComponentLocation` (`self.FREE`)))
    (set `self.TempLocation` (`SceneComponent.K2_GetComponentLocation` _piecetoswap))
    ;[1 1 1] Swap the 2 pieces
    (`SceneComponent.K2_SetWorldLocation` _piecetoswap (`self.LocationFreePlace`) false false)
    (`SceneComponent.K2_SetWorldLocation` (`self.FREE`) (`self.TempLocation`) false false)
    ;[1 1 1] Swap the pieces in the arrays
    (bind _asstatic_mesh_component (cast `StaticMeshComponent` (`self.PieceToSwap`)))
    (`KismetArrayLibrary.Array_Swap` (`self.ArrayPieces`) (`KismetArrayLibrary.Array_Find` (`self.ArrayPieces`) _asstatic_mesh_component) (`KismetArrayLibrary.Array_Find` (`self.ArrayPieces`) (`self.FREE`)))))

(fn `UserConstructionScript`
  ;[1 1 1] Create array with all pieces
  (bind _output_get (set `self.ArrayPiecesOrdered` (`|MakeArray` (`self.1`) (`self.2`) (`self.3`) (`self.4`) (`self.5`) (`self.6`) (`self.7`) (`self.8`) (`self.9`) (`self.10`) (`self.11`) (`self.12`) (`self.13`) (`self.14`) (`self.15`) (`self.FREE`))))
  ;[1 1 1] Create tab with all starting locations
  (for _array_element _output_get
    (`KismetArrayLibrary.Array_Add` (`self.Locations`) (`SceneComponent.K2_GetComponentLocation` _array_element)))
  ;[1 1 1] Create array with all pieces (Shuffle mmanually to have a functional solution)
  (bind _output_get_2 (set `self.ArrayPieces` (`|MakeArray` (`self.4`) (`self.14`) (`self.9`) (`self.5`) (`self.6`) (`self.13`) (`self.1`) (`self.7`) (`self.FREE`) (`self.8`) (`self.12`) (`self.15`) (`self.3`) (`self.11`) (`self.2`) (`self.10`))))
  ;[1 1 1] Shuffle pieces and display the pieces at their new places
  (for (_array_element_2 _array_index) _output_get_2
    (`SceneComponent.K2_SetWorldLocation` _array_element_2 (`|GetArrayItem` (`self.Locations`) _array_index) false false)))