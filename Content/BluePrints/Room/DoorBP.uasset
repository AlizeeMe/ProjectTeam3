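; Door Blueprint that swings open and closed when triggered while the first-person character is in range.
; A collision box sets a flag as the character enters and leaves, and OpenDoorEvent acts only while that flag is set.
; Each accepted call alternates, via a FlipFlop, between playing and reversing the OpenDoor timeline, which drives the yaw of the Scene component.
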(event `self.Door Collision Box.OnComponentEndOverlap`
  (params (OverlappedComponent :type "PrimitiveComponent Object Reference") (OtherActor :type "Actor Object Reference") (OtherComp :type "PrimitiveComponent Object Reference") (OtherBodyIndex :type Integer))
  (cast `/Game/FirstPersonBP/Blueprints/FirstPersonCharacter` OtherActor)
  (set `self.InsideCollisionBox` false))

(event `self.Door Collision Box.OnComponentBeginOverlap`
  (params (OverlappedComponent :type "PrimitiveComponent Object Reference") (OtherActor :type "Actor Object Reference") (OtherComp :type "PrimitiveComponent Object Reference") (OtherBodyIndex :type Integer) (bFromSweep :type Boolean) (SweepResult :type "HitResult Structure (by ref)"))
  (cast `/Game/FirstPersonBP/Blueprints/FirstPersonCharacter` OtherActor)
  (set `self.InsideCollisionBox` true))

(event `Open Door Event`
  (if (`self.InsideCollisionBox`)
    (`/Engine/EditorBlueprintResources/StandardMacros.FlipFlop`
      (:`A`
        (bind (_direction _dooropenamount) (`Timeline|Open Door` :!label _label)
          (:`Update`
            (`SceneComponent.K2_SetRelativeRotation` (`self.Scene`) (`KismetMathLibrary.MakeRotator` 0.0 0.0 _dooropenamount) false false))))
      (:`B`
        (goto _label :!via `Reverse`)))))

(fn `UserConstructionScript`)